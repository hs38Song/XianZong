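; BP_item is a pickup item actor whose mesh comes from the ItemModelToPlace variable, applied in the construction script.
; Its PickUp event prints a message and plays the Shrink timeline to scale the mesh toward zero.
; The sound, half-second delay and actor destruction all hang off the timeline's Update, so the sound fires on every update and destruction follows the first delay rather than timeline completion.
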(event `/Game/MyBlueprint/BPI_items.PickUp`
  (`KismetSystemLibrary.PrintString` "Item picked")
  (bind (_direction _newtrack_0) (`Timeline|Shrink`)
    (:`Update`
      (`SceneComponent.SetWorldScale3D` (`self.Item`) (`KismetMathLibrary.Conv_DoubleToVector` (`KismetMathLibrary.Lerp` 1.0 0.0 _newtrack_0)))
      (`GameplayStatics.PlaySound2D` "/Engine/VREditor/Sounds/UI/Object_PickUp.Object_PickUp" 1.0 1.0 0.0 null null)
      (`KismetSystemLibrary.Delay` 0.5)
      (`self.K2_DestroyActor`))))

(fn `UserConstructionScript`
  (`StaticMeshComponent.SetStaticMesh` (`self.Item`) (`self.ItemModelToPlace`)))