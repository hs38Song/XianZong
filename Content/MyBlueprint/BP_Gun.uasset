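; BP_Gun is a gun actor Blueprint that can fire bullets and be picked up.
; Fire spawns BP_Bullet at the Arrow component with sound and an attached muzzle flash, using the Interval flag and a two-second Delay as a cooldown.
; PickUp runs a Timeline that shrinks the Scoper component, with the pickup sound and delayed actor destruction both triggered from the Timeline's Update output.
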(event `Fire`
  (if (`self.Interval`)
    (`|SpawnActorFromClass` "/Game/MyBlueprint/BP_Bullet.BP_Bullet_C" (`SceneComponent.K2_GetComponentToWorld` (`self.Arrow`)) "Undefined" "MultiplyWithRoot" null null)
    (`GameplayStatics.PlaySoundAtLocation` "/Game/FPWeapon/Audio/FirstPersonTemplateWeaponFire02.FirstPersonTemplateWeaponFire02" (`self.K2_GetActorLocation`) (struct) 1.0 1.0 0.0 null null null null) ; Play firing sound
    (`NiagaraFunctionLibrary.SpawnSystemAttached` "/Game/ScifiWeapons/Effects/P_MuzzleFlash.P_MuzzleFlash" (`self.Arrow`) "None" (0.0 0.0 0.0) (struct) "KeepRelativeOffset")
    (set `self.Interval` false)
    (`KismetSystemLibrary.Delay` 2.0)
    (set `self.Interval` true)))

(event `/Game/MyBlueprint/BPI_items.PickUp`
  (`KismetSystemLibrary.PrintString` "Item picked")
  (bind (_direction _newtrack_0) (`Timeline|Timeline`)
    (:`Update`
      (`SceneComponent.SetWorldScale3D` (`self.Scoper`) (`KismetMathLibrary.Conv_DoubleToVector` (`KismetMathLibrary.Lerp` 1.0 0.0 _newtrack_0)))
      (`GameplayStatics.PlaySound2D` "/Engine/VREditor/Sounds/UI/Object_PickUp.Object_PickUp" 1.0 1.0 0.0 null null)
      (`KismetSystemLibrary.Delay` 0.3)
      (`self.K2_DestroyActor`))))

(fn `UserConstructionScript`)