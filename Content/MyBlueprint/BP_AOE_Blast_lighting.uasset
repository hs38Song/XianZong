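; BP_AOE_Blast_lighting is a delayed area-of-effect blast actor, named as a lighting variant.
; On BeginPlay it runs the parent logic, spawns a ground-marker-sized decal at its location with an engine debug material, waits DelayBefore, then calls Trigger.
; The blast effect itself is not defined in this graph.
; After triggering, a validity check on the decal leads to destroying DefaultSceneRoot, not the decal component.
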(event `self.ReceiveBeginPlay`
  (`parent.ReceiveBeginPlay`)
  (bind _returnvalue (`GameplayStatics.SpawnDecalAtLocation` "/Engine/EngineDebugMaterials/LevelColorationUnlitMaterial.LevelColorationUnlitMaterial" (25.0 256.0 256.0) (`self.K2_GetActorLocation`)))
  (`KismetSystemLibrary.Delay` (`self.DelayBefore`))
  (`self.Trigger`)
  (`/Engine/EditorBlueprintResources/StandardMacros.IsValid` _returnvalue
    (:`Is Valid`
      (`ActorComponent.K2_DestroyComponent` (`self.DefaultSceneRoot`)))))

(fn `UserConstructionScript`
  (`parent.UserConstructionScript`))