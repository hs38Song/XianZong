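; BP_AOE_Base is a base area-of-effect actor that finds third-person character pawns within a radius of itself.
; Trigger runs the effect, either automatically shortly after BeginPlay or when called.
; A sphere overlap, optionally ignoring the instigator and drawing a debug sphere, calls the OnAOEOverlapActor dispatcher for each hit.
; Debug prints remain, and a looping timer node is left unwired.
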(event `self.ReceiveBeginPlay`
  (if (`self.TriggerOnBeginPlay`)
    (`KismetSystemLibrary.Delay` 0.2)
    (`self.Trigger`)))

(event `Trigger`
  (`self.Spawn AOE`))

(event `Spawn AOE`
  (bind _returnvalue (`self.K2_GetActorLocation`))
  (bind _radius (`self.Radius`))
  (`KismetSystemLibrary.PrintString` "Hello")
  (if (`self.DrawDebug`)
    (`KismetSystemLibrary.DrawDebugSphere` _returnvalue _radius 12 (struct :`R` 1.0 :`B` 0.140964 :`A` 1.0) 1.0 1.0))
  (bind _outactors (`KismetSystemLibrary.SphereOverlapActors` _returnvalue _radius (`|MakeArray` "ObjectTypeQuery3" :!type "EObjectTypeQuery Enum") "/Game/ThirdPerson/Blueprints/BP_ThirdPersonCharacter.BP_ThirdPersonCharacter_C" (select `bool` (`self.IgnoreInstigator`) :`true` (`|MakeArray` (`self.GetInstigator`) :!type "Actor Object Reference"))))
  (for _array_element _outactors
    (`self.OnAOEOverlapActor` _array_element)
    (`KismetSystemLibrary.PrintString` (`KismetSystemLibrary.GetDisplayName` _array_element))))

(fn `UserConstructionScript`)