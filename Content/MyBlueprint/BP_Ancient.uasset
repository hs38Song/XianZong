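; BP_Ancient is a boss enemy character that takes damage from player shots and adds score to the game mode when killed.
; Each Tick updates its widget health bar and rotates it to face the camera.
; Generic damage and capsule hits feed ReduceHealth; bullets hit hard, while first-person projectiles hit lightly and briefly freeze movement and animation.
; At zero health it emits steam, ragdolls the mesh, then calls Death after a delay.
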(event `self.ReceiveTick`
  (params (DeltaSeconds :type "Float (single-precision)"))
  (bind _health_barwidget (`self.Health BarWidget`))
  (bind _asenemy_health_bar (cast `/Game/CityofBrass_Enemies/EnemyHealthBar` (`WidgetComponent.GetWidget` (`self.Health BarWidget`))))
  (`ProgressBar.SetPercent` (`/Game/CityofBrass_Enemies/EnemyHealthBar.HealthBar` _asenemy_health_bar) (/ (`self.Health`) 500.0))
  (`SceneComponent.K2_SetWorldRotation` _health_barwidget (`KismetMathLibrary.FindLookAtRotation` (`SceneComponent.K2_GetComponentLocation` _health_barwidget) (`SceneComponent.K2_GetComponentLocation` (`PlayerCameraManager.TransformComponent` (`GameplayStatics.GetPlayerCameraManager` 0)))) false false))

(event `Death`
  (`KismetSystemLibrary.PrintString` "Boss Eliminated")
  (bind _asgm_xiang_zong_game_mode (cast `/Game/MyBlueprint/GM_XiangZongGameMode` (`GameplayStatics.GetGameMode`))
    (:`then`
      (`/Game/MyBlueprint/GM_XiangZongGameMode.AddScore` _asgm_xiang_zong_game_mode)
      (`PrimitiveComponent.SetSimulatePhysics` (`self.CapsuleComponent`) true))
    (:`CastFailed`
      (`KismetSystemLibrary.PrintString` "???"))))

(event `ReduceHealth`
  (params (Damage :type "Float (double-precision)"))
  (bind _output_get (set `self.Health` (- (`self.Health`) Damage)))
  (if (<= _output_get 0.0)
    (`GameplayStatics.SpawnEmitterAtLocation` "/Game/StarterContent/Particles/P_Steam_Lit.P_Steam_Lit")
    (`PrimitiveComponent.SetSimulatePhysics` (`self.Mesh`) true)
    (`MovementComponent.StopMovementImmediately` (`self.CharacterMovement`))
    (`KismetSystemLibrary.Delay` 1.0)
    (`self.Death`)))

(event `self.ReceiveAnyDamage`
  (params (Damage :type "Float (single-precision)") (DamageType :type "DamageType Object Reference") (InstigatedBy :type "Controller Object Reference") (DamageCauser :type "Actor Object Reference"))
  (`self.ReduceHealth` Damage))

(event `Freeze`
  (`CharacterMovementComponent.SetMovementMode` (`self.CharacterMovement`) "MOVE_None" 0)
  (`SkeletalMeshComponent.Stop` (`self.Mesh`))
  (`KismetSystemLibrary.Delay` 1.0)
  (`CharacterMovementComponent.SetMovementMode` (`self.CharacterMovement`) "MOVE_Walking" 0)
  (`SkeletalMeshComponent.PlayAnimation` (`self.Mesh`) "/Game/CityofBrass_Enemies/Meshes/Enemy/Corpse/animation/Corpse_Run_Forward.Corpse_Run_Forward" true))

(event `self.CapsuleComponent.OnComponentHit`
  (params (HitComponent :type "PrimitiveComponent Object Reference") (OtherActor :type "Actor Object Reference") (OtherComp :type "PrimitiveComponent Object Reference") (NormalImpulse :type "Vector Structure") (Hit :type "HitResult Structure (by ref)"))
  (cast `/Game/MyBlueprint/BP_Bullet` OtherActor
    (:`then`
      (`self.ReduceHealth` 40.0)
      (`GameplayStatics.PlaySound2D` "/Game/StarterContent/Audio/Collapse01.Collapse01" 1.0 1.0 0.0 null null))
    (:`CastFailed`
      (cast `/Game/FirstPerson/Blueprints/BP_FirstPersonProjectile` OtherActor)
      (`self.ReduceHealth` 5.0)
      (`GameplayStatics.PlaySound2D` "/Game/StarterContent/Audio/Collapse01.Collapse01" 1.0 1.0 0.0 null null)
      (`self.Freeze`))))

(fn `UserConstructionScript`)