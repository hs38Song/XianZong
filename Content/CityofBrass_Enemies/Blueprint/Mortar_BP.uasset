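; Mortar enemy that repeatedly lobs projectiles at the player from BeginPlay on a timed loop.
; Each shot leads the player by velocity and distance, using a suggested custom arc for launch velocity; the randomized offset only feeds a debug sphere.
; Touching the capsule damages the player and knocks them back.
; Touching the head bounces the player upward, destroys the mortar and awards score.
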(event `self.Capsule.OnComponentBeginOverlap`
  (params (OverlappedComponent :type "PrimitiveComponent Object Reference") (OtherActor :type "Actor Object Reference") (OtherComp :type "PrimitiveComponent Object Reference") (OtherBodyIndex :type Integer) (bFromSweep :type Boolean) (SweepResult :type "HitResult Structure (by ref)"))
  (bind _asbp_learning_kit_player_character (cast `/Game/LearningKit_Games/Blueprints/BP_LearningKit_PlayerCharacter` OtherActor))
  (`GameplayStatics.ApplyDamage` _asbp_learning_kit_player_character 10.0)
  (`GameplayStatics.PlaySoundAtLocation` "/Game/LearningKit_Games/Sound/block_hit.block_hit" (`self.K2_GetActorLocation`) (struct) 1.0 1.0 0.0 null null null null)
  (`Character.LaunchCharacter` _asbp_learning_kit_player_character (`KismetMathLibrary.MakeVector` (.x (* (`self.GetActorForwardVector` _asbp_learning_kit_player_character) (-1000.0 -1000.0 0.0))) (.y (* (`self.GetActorForwardVector` _asbp_learning_kit_player_character) (-1000.0 -1000.0 0.0))) (+ (.z (* (`self.GetActorForwardVector` _asbp_learning_kit_player_character) (-1000.0 -1000.0 0.0))) 500.0)) false false))

(event `ReFire`
  (`self.EventFire` (`GameplayStatics.GetPlayerCharacter` 0) :!label _label))

(event `self.ReceiveBeginPlay`
  (goto _label))

(event `EventFire`
  (params (`Target Actor` :type "Actor Object Reference"))
  (`/Engine/EditorBlueprintResources/StandardMacros.IsValid` `Target Actor`
    (:`Is Valid`
      (bind _desiredvelocity (`self.MortarPredictionFunction` `Target Actor`))
      (set `self.DesiredVelocity` _desiredvelocity)
      (bind _returnvalue (`|SpawnActorFromClass` "/Game/LearningKit_Games/Blueprints/Mortar_Projectile.Mortar_Projectile_C" (`KismetMathLibrary.MakeTransform` (`SceneComponent.K2_GetComponentLocation` (`self.Arrow`))) "Undefined" "MultiplyWithRoot" null null))
      (`/Engine/EditorBlueprintResources/StandardMacros.IsValid` _returnvalue
        (:`Is Valid`
          (`ProjectileMovementComponent.SetVelocityInLocalSpace` (`/Game/LearningKit_Games/Blueprints/Mortar_Projectile.ProjectileMovement` _returnvalue) (`self.DesiredVelocity`))
          (`KismetSystemLibrary.Delay` 2.0)
          (`self.ReFire`))
        (:`Is Not Valid`
          (`self.ReFire`))))))

(event `self.head.OnComponentBeginOverlap`
  (params (OverlappedComponent :type "PrimitiveComponent Object Reference") (OtherActor :type "Actor Object Reference") (OtherComp :type "PrimitiveComponent Object Reference") (OtherBodyIndex :type Integer) (bFromSweep :type Boolean) (SweepResult :type "HitResult Structure (by ref)"))
  (bind _asbp_learning_kit_player_character (cast `/Game/LearningKit_Games/Blueprints/BP_LearningKit_PlayerCharacter` OtherActor))
  (`GameplayStatics.PlaySoundAtLocation` "/Game/LearningKit_Games/Sound/eliminate_enemy.eliminate_enemy" (`self.K2_GetActorLocation`) (struct) 1.0 1.0 0.0 null null null null)
  (`Character.LaunchCharacter` _asbp_learning_kit_player_character (0.0 0.0 1000.0) false false)
  (`self.K2_DestroyActor`)
  (`/Game/LearningKit_Games/Blueprints/BP_LearningKit_PlayerCharacter.IncreaseScore` _asbp_learning_kit_player_character 20))

(fn `addVectorRandomness`
  (params (Vector :type "Vector Structure") (Randomness :type "Float (double-precision)" :default 1000.0) (X :type Boolean :default true) (Y :type Boolean :default true) (Z :type Boolean :default true))
  (returns (`Return Vector` :type "Vector Structure"))
  (bind _x (.x Vector))
  (bind _y (.y Vector))
  (bind _z (.z Vector))
  (bind _returnvalue (* Randomness -1.0))
  (return (`KismetMathLibrary.MakeVector_NetQuantize` (`KismetMathLibrary.SelectFloat` _x (+ (`KismetMathLibrary.RandomFloatInRange` _returnvalue Randomness) _x) X) (`KismetMathLibrary.SelectFloat` _y (+ (`KismetMathLibrary.RandomFloatInRange` _returnvalue Randomness) _y) Y) (`KismetMathLibrary.SelectFloat` _z (+ (`KismetMathLibrary.RandomFloatInRange` _returnvalue Randomness) _z) Z))))

(fn `MortarPredictionFunction`
  (params (TargetActor :type "Actor Object Reference"))
  (returns (DesiredVelocity :type "Vector Structure"))
  (locals (ActorVelocity :type "Vector Structure") (ActorLocation :type "Vector Structure"))
  (bind _returnvalue (+ (`local.ActorLocation`) (* (`KismetMathLibrary.SafeDivide` (`KismetMathLibrary.Vector_Distance` (`local.ActorLocation`) (`self.K2_GetActorLocation`)) 1000.0) (`local.ActorVelocity`))))
  (set `local.ActorVelocity` (`self.GetVelocity` TargetActor))
  (set `local.ActorLocation` (`self.K2_GetActorLocation` TargetActor))
  (`KismetSystemLibrary.DrawDebugSphere` _returnvalue 10.0 4 (struct :`R` 0.04173 :`G` 1.0 :`B` 0.050982 :`A` 1.0) 10.0 2.0)
  (`KismetSystemLibrary.DrawDebugSphere` (`self.addVectorRandomness` _returnvalue) 10.0 4 (struct :`R` 1.0 :`B` 0.040184 :`A` 1.0) 10.0 2.0)
  (bind (_outlaunchvelocity _returnvalue_2) (`GameplayStatics.SuggestProjectileVelocity_CustomArc` (`SceneComponent.K2_GetComponentLocation` (`self.Arrow`)) _returnvalue))
  (if _returnvalue_2
    (return _outlaunchvelocity)))

(fn `UserConstructionScript`)