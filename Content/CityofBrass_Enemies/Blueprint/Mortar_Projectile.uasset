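; Mortar projectile Blueprint that explodes on hit and then destroys itself.
; Every hit applies radial damage around the impact point, plays an explosion sound and spawns a Niagara burst.
; A direct hit on the learning kit player character also sets its IsHit flag, deals extra damage and launches it along the reversed horizontal hit normal with an added upward boost.
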(event `self.ReceiveHit`
  (params (MyComp :type "PrimitiveComponent Object Reference") (Other :type "Actor Object Reference") (OtherComp :type "PrimitiveComponent Object Reference") (bSelfMoved :type Boolean) (HitLocation :type "Vector Structure") (HitNormal :type "Vector Structure") (NormalImpulse :type "Vector Structure") (Hit :type "HitResult Structure (by ref)"))
  (`GameplayStatics.ApplyRadialDamageWithFalloff` :`BaseDamage` 50.0 :`MinimumDamage` 50.0 :`Origin` HitLocation :`DamageInnerRadius` 50.0 :`DamageOuterRadius` 200.0 :`DamageFalloff` 1.0 :`DamageCauser` null :`InstigatedByController` null)
  (`GameplayStatics.PlaySoundAtLocation` "/Game/LearningKit_Games/Sound/explosion.explosion" HitLocation (struct) 0.2 1.0 0.0 null null null null)
  (`NiagaraFunctionLibrary.SpawnSystemAtLocation` "/Game/LearningKit_Robots/VFX/Bursts/NS_Burst_Simple.NS_Burst_Simple" HitLocation)
  (bind _asbp_learning_kit_player_character (cast `/Game/LearningKit_Games/Blueprints/BP_LearningKit_PlayerCharacter` Other)
    (:`then`
      (set `/Game/LearningKit_Games/Blueprints/BP_LearningKit_PlayerCharacter.IsHit` true _asbp_learning_kit_player_character)
      (`GameplayStatics.ApplyDamage` _asbp_learning_kit_player_character 15.0)
      (`Character.LaunchCharacter` _asbp_learning_kit_player_character (`KismetMathLibrary.MakeVector` (.x (* HitNormal (-1000.0 -1000.0 100.0))) (.y (* HitNormal (-1000.0 -1000.0 100.0))) (+ (.z (* HitNormal (-1000.0 -1000.0 100.0))) 100.0)) false false)
      (`self.K2_DestroyActor`))
    (:`CastFailed`
      (`self.K2_DestroyActor`))))

(fn `UserConstructionScript`)