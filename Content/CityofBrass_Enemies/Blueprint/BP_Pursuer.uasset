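; BP_Pursuer is a melee enemy that either roams nearby points or chases the player, chosen by AIState at BeginPlay.
; The looping chase plays an attack on arrival, then deals damage with effects if the player is still close.
; Bullet and first-person projectile hits reduce health and ragdoll it before destruction at zero; non-lethal projectile hits also briefly freeze it.
; Tick updates a health bar widget that faces the camera.
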(event `self.ReceiveTick`
  (params (DeltaSeconds :type "Float (single-precision)"))
  (bind _health_barwidget (`self.Health BarWidget`))
  (bind _asenemy_health_bar (cast `/Game/CityofBrass_Enemies/EnemyHealthBar` (`WidgetComponent.GetWidget` (`self.Health BarWidget`))))
  (`ProgressBar.SetPercent` (`/Game/CityofBrass_Enemies/EnemyHealthBar.HealthBar` _asenemy_health_bar) (/ (`self.Health`) 100.0))
  (`SceneComponent.K2_SetWorldRotation` _health_barwidget (`KismetMathLibrary.FindLookAtRotation` (`SceneComponent.K2_GetComponentLocation` _health_barwidget) (`SceneComponent.K2_GetComponentLocation` (`PlayerCameraManager.TransformComponent` (`GameplayStatics.GetPlayerCameraManager` 0)))) false false))

(event `Freeze`
  (`CharacterMovementComponent.SetMovementMode` (`self.CharacterMovement`) "MOVE_None" 0)
  (`SkeletalMeshComponent.Stop` (`self.Mesh`))
  (`KismetSystemLibrary.Delay` 1.0)
  (`CharacterMovementComponent.SetMovementMode` (`self.CharacterMovement`) "MOVE_Walking" 0)
  (`SkeletalMeshComponent.PlayAnimation` (`self.Mesh`) "/Game/CityofBrass_Enemies/Meshes/Enemy/Corpse/animation/Corpse_Run_Forward.Corpse_Run_Forward" true))

(event `Roam`
  (`|AIMoveTo` self (`NavigationSystemV1.K2_GetRandomReachablePointInRadius` (`self.K2_GetActorLocation` self) 50.0 null null) null
    (:`OnSuccess`
      (`KismetSystemLibrary.Delay` 0.5)
      (`self.Roam`))))

(event `self.ReceiveBeginPlay`
  (switch `/Game/CityofBrass_Enemies/Blueprint/EAIState` (`self.AIState`)
    (:`NewEnumerator0`
      (`self.Roam` self :!label _label))
    (:`NewEnumerator1`
      (goto _label))
    (:`NewEnumerator2`
      (`self.ChasePlayer`))))

(event `ChasePlayer`
  (`|AIMoveTo` self (0.0 0.0 0.0) (`GameplayStatics.GetPlayerCharacter` 0)
    (:`OnSuccess`
      (`SkeletalMeshComponent.PlayAnimation` (`self.Mesh`) "/Game/CityofBrass_Enemies/Meshes/Enemy/Corpse/animation/Corpse_Alert_Attack_Slow.Corpse_Alert_Attack_Slow" false)
      (`KismetSystemLibrary.Delay` 0.9)
      (if (>= (`KismetMathLibrary.Vector_Distance` (`self.K2_GetActorLocation`) (`self.K2_GetActorLocation` (`GameplayStatics.GetPlayerCharacter` 0))) 300.0)
        (`SkeletalMeshComponent.PlayAnimation` (`self.Mesh`) "/Game/CityofBrass_Enemies/Meshes/Enemy/Corpse/animation/Corpse_Run_Forward.Corpse_Run_Forward" true)
        (`self.ChasePlayer`)
        (else
          (bind _returnvalue (`GameplayStatics.SpawnEmitterAtLocation` "/Engine/Tutorial/SubEditors/TutorialAssets/TutorialParticleSystem.TutorialParticleSystem" (`self.K2_GetActorLocation` self)))
          (`GameplayStatics.PlaySoundAtLocation` null (`self.K2_GetActorLocation`) (struct) 1.0 1.0 0.0 null null null null)
          (`GameplayStatics.ApplyDamage` (`GameplayStatics.GetPlayerCharacter` 0) 20.0)
          (`KismetSystemLibrary.Delay` 0.5)
          (`SkeletalMeshComponent.PlayAnimation` (`self.Mesh`) "/Game/CityofBrass_Enemies/Meshes/Enemy/Corpse/animation/Corpse_Run_Forward.Corpse_Run_Forward" true)
          (`ActorComponent.K2_DestroyComponent` _returnvalue)
          (`self.ChasePlayer`))))
    (:`OnFail`
      (`KismetSystemLibrary.Delay` 0.05)
      (`self.ChasePlayer`))))

(event `self.CapsuleComponent.OnComponentHit`
  (params (HitComponent :type "PrimitiveComponent Object Reference") (OtherActor :type "Actor Object Reference") (OtherComp :type "PrimitiveComponent Object Reference") (NormalImpulse :type "Vector Structure") (Hit :type "HitResult Structure (by ref)"))
  (cast `/Game/MyBlueprint/BP_Bullet` OtherActor
    (:`then`
      (`self.ReduceHealth` 40.0)
      (`GameplayStatics.PlaySound2D` "/Game/StarterContent/Audio/Collapse01.Collapse01" 1.0 1.0 0.0 null null)
      (if (<= (`self.Health`) 0.0)
        (`PrimitiveComponent.SetSimulatePhysics` (`self.Mesh`) true)
        (`KismetSystemLibrary.Delay` 2.0)
        (`self.K2_DestroyActor`)))
    (:`CastFailed`
      (cast `/Game/FirstPerson/Blueprints/BP_FirstPersonProjectile` OtherActor)
      (`self.ReduceHealth` 5.0)
      (`GameplayStatics.PlaySound2D` "/Game/StarterContent/Audio/Collapse01.Collapse01" 1.0 1.0 0.0 null null)
      (if (<= (`self.Health`) 0.0)
        (`PrimitiveComponent.SetSimulatePhysics` (`self.Mesh`) true)
        (`KismetSystemLibrary.Delay` 2.0)
        (`self.K2_DestroyActor`)
        (else
          (`self.Freeze`))))))

(event `ReduceHealth`
  (params (Damage :type "Float (double-precision)"))
  (set `self.Health` (- (`self.Health`) Damage)))

(fn `UserConstructionScript`)