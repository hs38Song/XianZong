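; Spline_Enemy is an enemy that hurts the player on contact and can be eliminated through its Head collider.
; A hit against the player character applies damage, plays a block sound and launches them away along the hit normal with an upward boost.
; A player overlap with Head plays an elimination sound, bounces the player upward, destroys the enemy and increases the player's score.
; No spline movement logic appears in its graphs.
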(event `self.ReceiveHit`
  (params (MyComp :type "PrimitiveComponent Object Reference") (Other :type "Actor Object Reference") (OtherComp :type "PrimitiveComponent Object Reference") (bSelfMoved :type Boolean) (HitLocation :type "Vector Structure") (HitNormal :type "Vector Structure") (NormalImpulse :type "Vector Structure") (Hit :type "HitResult Structure (by ref)"))
  (bind _asbp_learning_kit_player_character (cast `/Game/LearningKit_Games/Blueprints/BP_LearningKit_PlayerCharacter` Other))
  (`GameplayStatics.ApplyDamage` _asbp_learning_kit_player_character 15.0)
  (`GameplayStatics.PlaySoundAtLocation` "/Game/LearningKit_Games/Sound/block_hit.block_hit" (`self.K2_GetActorLocation` Other) (struct) 1.0 1.0 0.0 null null null null)
  (`Character.LaunchCharacter` _asbp_learning_kit_player_character (`KismetMathLibrary.MakeVector` (.x (* HitNormal (-2000.0 -2000.0 0.0))) (.y (* HitNormal (-2000.0 -2000.0 0.0))) (+ (.z (* HitNormal (-2000.0 -2000.0 0.0))) 500.0)) false false))

(event `self.head.OnComponentBeginOverlap`
  (params (OverlappedComponent :type "PrimitiveComponent Object Reference") (OtherActor :type "Actor Object Reference") (OtherComp :type "PrimitiveComponent Object Reference") (OtherBodyIndex :type Integer) (bFromSweep :type Boolean) (SweepResult :type "HitResult Structure (by ref)"))
  (bind _asbp_learning_kit_player_character (cast `/Game/LearningKit_Games/Blueprints/BP_LearningKit_PlayerCharacter` OtherActor))
  (`GameplayStatics.PlaySoundAtLocation` "/Game/LearningKit_Games/Sound/eliminate_enemy.eliminate_enemy" (`self.K2_GetActorLocation`) (struct) 1.0 1.0 0.0 null null null null)
  (`Character.LaunchCharacter` _asbp_learning_kit_player_character (0.0 0.0 1000.0) false false)
  (`self.K2_DestroyActor`)
  (`/Game/LearningKit_Games/Blueprints/BP_LearningKit_PlayerCharacter.IncreaseScore` _asbp_learning_kit_player_character 15))

(fn `UserConstructionScript`)