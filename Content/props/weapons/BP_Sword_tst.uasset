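; BP_Sword_tst is a sword pickup actor, apparently a test asset, that shrinks away and destroys itself when picked up.
; Its PickUp event prints a debug message and plays a timeline that lerps the WeaponModel's world scale from one toward zero.
; The pickup sound and delayed destroy hang off the timeline's Update pin, so the sound fires on every update until the short delay removes the actor.
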(event `/Game/MyBlueprint/BPI_items.PickUp`
  (`KismetSystemLibrary.PrintString` "Item picked")
  (bind (_direction _newtrack_0) (`Timeline|Timeline`)
    (:`Update`
      (`SceneComponent.SetWorldScale3D` (`self.WeaponModel`) (`KismetMathLibrary.Conv_DoubleToVector` (`KismetMathLibrary.Lerp` 1.0 0.0 _newtrack_0)))
      (`GameplayStatics.PlaySound2D` "/Engine/VREditor/Sounds/UI/Object_PickUp.Object_PickUp" 1.0 1.0 0.0 null null)
      (`KismetSystemLibrary.Delay` 0.3)
      (`self.K2_DestroyActor`))))

(fn `UserConstructionScript`
  (`parent.UserConstructionScript`))